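; Live Link remap asset that translates ARKit-style face capture curve names into the Fcl_-prefixed morph target names of the Shenjingxin character.
; It overrides GetRemappedCurveName with a single name switch covering a subset of eye, jaw, mouth and brow curves, passing all other names through unchanged.
; For paired shapes such as blink, smile and frown, only the left-side curve drives the combined target.
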(fn GetRemappedCurveName
  (params (CurveName :type Name :default "None"))
  (switch name CurveName
    (:Default
      (return CurveName))
    (:EyeBlinkLeft
      (return "Fcl_EYE_Close"))
    (:JawOpen
      (return "Fcl_MTH_A"))
    (:MouthClose
      (return "Fcl_MTH_Close"))
    (:MouthFunnel
      (return "Fcl_MTH_O"))
    (:MouthPuncker
      (return "Fcl_MTH_U"))
    (:MouthLeft
      (return "Fcl_MTH_I"))
    (:MouthSmileLeft
      (return "Fcl_MTH_Fun"))
    (:MouthFrownLeft
      (return "Fcl_MTH_Angry"))
    (:MouthStretchLeft
      (return "Fcl_MTH_E"))
    (:BrowDownLeft
      (return "Fcl_BRW_Angry"))
    (:BrowInnerUp
      (return "Fcl_BRW_Joy"))))