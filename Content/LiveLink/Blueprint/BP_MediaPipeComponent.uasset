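; Actor Blueprint that runs MediaPipe Holistic webcam capture with an on-screen control UI and camera preview.
; BeginPlay shows the mouse cursor, creates WB_LiveLinkMain, and binds its start/stop buttons to the MediaPipeHolistic camera.
; When the video texture is created, it feeds a dynamic M_Webcamera material and anchors the preview bottom-right.
; Tick shows the preview only while MediaPipe is running.
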(event Custom|OnVideoTextureCreated_Event
  (params (NewTexture :type Texture%202D%20Object%20Reference) (TextureWidth :type Integer) (TextureHeight :type Integer))
  ;[1 1 1] 回显图像
  (Class|MediaPipeUtils|AnchorWidgetinCanvas (Variables|/Game/LiveLink/UMG/WB_LiveLinkMain.WB_LiveLinkMain_C|GetWebCamera (Variables|Default|GetWB_LiveLinkMain)) TextureWidth TextureHeight 0.3 0.3 "BottomRight")
  (Rendering|Material|SetTextureParameterValue (Variables|Default|GetM_Webcamera) "Texture" NewTexture))

(event Custom|StartCapture_Event
  ;[1 1 1] 打开1号摄像头
  (Class|MediaPipeHolisticComponent|StartCamera (Variables|Default|GetMediaPipeHolistic) 1 1280 720 30))

(event Custom|StopCapture_Event
  (Audio|Components|Audio|Stop (Variables|Default|GetMediaPipeHolistic)))

(event EventBeginPlay
  (Utilities|FlowControl|Sequence
    (:then_0
      (Variables|/Script/Engine.PlayerController|SetbShowMouseCursor (Game|GetPlayerController 0) true)
      (bind _returnvalue (UserInterface|CreateWidget "/Game/LiveLink/UMG/WB_LiveLinkMain.WB_LiveLinkMain_C"))
      (bind _output_get (Variables|Default|SetWB_LiveLinkMain _returnvalue))
      (UserInterface|Viewport|AddtoViewport _output_get 0))
    (:then_1
      (EventDispatchers|AssignOnClicked (Variables|/Game/LiveLink/UMG/WB_LiveLinkMain.WB_LiveLinkMain_C|GetButton_StartCapture (Variables|Default|GetWB_LiveLinkMain)) (delegate Custom|StartCapture_Event)))
    (:then_2
      ;[1 1 1] 回显图像
      (bind _returnvalue_2 (Rendering|Material|CreateDynamicMaterialInstance "/Game/LiveLink/Material/M_Webcamera.M_Webcamera" "None" "None" :!class /Script/Engine.KismetMaterialLibrary))
      (Variables|Default|SetM_Webcamera _returnvalue_2)
      (Class|Image|SetBrushfromMaterial (Variables|/Game/LiveLink/UMG/WB_LiveLinkMain.WB_LiveLinkMain_C|GetWebCamera (Variables|Default|GetWB_LiveLinkMain)) (Variables|Default|GetM_Webcamera)))
    (:then_3
      (EventDispatchers|AssignOnVideoTextureCreated (Variables|Default|GetMediaPipeHolistic) (delegate Custom|OnVideoTextureCreated_Event)))
    (:then_4
      (EventDispatchers|AssignOnClicked (Variables|/Game/LiveLink/UMG/WB_LiveLinkMain.WB_LiveLinkMain_C|GetButton_StopCapture (Variables|Default|GetWB_LiveLinkMain)) (delegate Custom|StopCapture_Event)))))

(event EventTick
  (params (DeltaSeconds :type Float%20%28single-precision%29))
  (bind _wb_livelinkmain (Variables|Default|GetWB_LiveLinkMain))
  (bind _webcamera (Variables|/Game/LiveLink/UMG/WB_LiveLinkMain.WB_LiveLinkMain_C|GetWebCamera _wb_livelinkmain))
  (if (Class|MediaPipeHolisticComponent|IsRunning (Variables|Default|GetMediaPipeHolistic))
    (Widget|SetVisibility _webcamera "Visible")
    (else
      (Widget|SetVisibility _webcamera "Collapsed"))))

(fn ConstructionScript)